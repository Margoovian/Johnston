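; Master weapon Blueprint that handles hitscan firing, ammo and reloading for the rifle, pistol and grenade launcher.
; Shoot decrements and prints ammo, traces unless the player is reloading, and gates fire rate with a delay.
; A spread-offset camera trace finds the aim point, then a muzzle trace follows; both only draw debug lines, without damage.
; Animations are chosen by hard-coded class checks, and Reload refills ammo after a delay.
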(event Custom|Shoot
  (bind _self self)
  (bind _gun (Variables|Components|GetGun))
  (bind _returnvalue (Utilities|GetClass _self))
  (if (not (Variables|Default|GetShot))
    (if (> (Variables|Default|GetAmmoCount) 0)
      (CallFunction|AmmoCheck)
      (if (not (Variables|/Game/Character/PlayerT.PlayerT_C|GetIsReloading (.AsPlayer%20T (Utilities|Casting|CastToPlayerT (Game|GetPlayerCharacter 0)))))
        (CallFunction|LineTrace)
        (if (== _returnvalue "/Game/Weapons/AssultRifle_Weapon.AssultRifle_Weapon_C")
          (Components|Animation|PlayAnimation _gun "/Game/Weapons/SciFiWeapDark/Weapons/Anims/Fire_Rifle_W.Fire_Rifle_W" false)
          (Variables|Default|SetShot true :!label _label)
          (Utilities|FlowControl|Delay (Variables|Default|GetShootingDelay))
          (Variables|Default|SetShot false)
          (elif (== _returnvalue "/Game/Weapons/Pistol_Weapon.Pistol_Weapon_C")
            (Components|Animation|PlayAnimation _gun "/Game/Weapons/SciFiWeapDark/Weapons/Anims/Fire_Pistol_W.Fire_Pistol_W" false)
            (goto _label)
            (elif (== _returnvalue "/Game/Weapons/GrenadeLauncher_Weapon.GrenadeLauncher_Weapon_C")
              (Components|Animation|PlayAnimation _gun "/Game/Weapons/SciFiWeapDark/Weapons/Anims/Fire_GrenadeLauncher_W.Fire_GrenadeLauncher_W" false)
              (goto _label)))))
      (else
        (Audio|PlaySoundatLocation "/Game/Weapons/SciFiWeapDark/Sound/Rifle/Wavs/Rifle_Whip01.Rifle_Whip01" (Transformation|GetWorldLocation (Variables|Components|GetGun)) "0, 0, 0" 1.0 1.0 0.0 0 0 0)))))

(event Custom|Reload
  (bind _self self)
  (bind _gun (Variables|Components|GetGun))
  (bind _returnvalue (Utilities|GetClass _self))
  (if (== _returnvalue "/Game/Weapons/AssultRifle_Weapon.AssultRifle_Weapon_C")
    (Components|Animation|PlayAnimation _gun "/Game/Weapons/SciFiWeapDark/Weapons/Anims/Reload_Rifle_Hip_W.Reload_Rifle_Hip_W" false)
    (Utilities|FlowControl|Delay (Variables|Default|GetReloadTime) :!label _label)
    (Variables|Default|SetAmmoCount (Variables|Default|GetMaxAmmo))
    (elif (== _returnvalue "/Game/Weapons/Pistol_Weapon.Pistol_Weapon_C")
      (Components|Animation|PlayAnimation _gun "/Game/Weapons/SciFiWeapDark/Weapons/Anims/Reload_Pistol_W.Reload_Pistol_W" false)
      (goto _label)
      (elif (== _returnvalue "/Game/Weapons/GrenadeLauncher_Weapon.GrenadeLauncher_Weapon_C")
        (Components|Animation|PlayAnimation _gun "/Game/Weapons/SciFiWeapDark/Weapons/Anims/Reload_GrenadeLauncher_W.Reload_GrenadeLauncher_W" false)
        (goto _label)))))

(fn ConstructionScript
  (bind _output_get (Variables|Default|SetMaxAmmo (Variables|Default|GetMaxAmmo)))
  (Variables|Default|SetAmmoCount _output_get)
  (Variables|Default|SetReloadTime (Variables|Default|GetReloadTime)))

(fn AmmoCheck
  (Math|Integer|DecrementInt (Variables|Default|GetAmmoCount)
    (:%20%20
      (if (not (Variables|/Game/Character/PlayerT.PlayerT_C|GetIsReloading (.AsPlayer%20T (Utilities|Casting|CastToPlayerT (Game|GetPlayerCharacter 0)))))
        (Development|PrintString (Utilities|String|ToString(Integer) (Variables|Default|GetAmmoCount)))))))

(fn LineTrace
  (bind _returnvalue (Game|GetPlayerCharacter 0))
  (bind _bulletspread (Variables|Default|GetBulletSpread))
  (bind _returnvalue_2 (* _bulletspread -1.0))
  (bind _asplayer_t (Utilities|Casting|CastToPlayerT _returnvalue))
  (bind _camera (Variables|/Game/Character/PlayerT.PlayerT_C|GetCamera _asplayer_t))
  (bind _returnvalue_3 (Transformation|GetWorldLocation _camera))
  (bind _outhit (Collision|LineTraceByChannel _returnvalue_3 (+ (+ (* (Math|Vector|GetForwardVector _camera) (Variables|Default|GetBulletFalloff)) _returnvalue_3) (Math|Vector|MakeVector (Math|Random|RandomFloatinRange _returnvalue_2 _bulletspread) (Math|Random|RandomFloatinRange _returnvalue_2 _bulletspread) (Math|Random|RandomFloatinRange _returnvalue_2 _bulletspread))) "TraceTypeQuery1" false 0 "ForDuration" true "(R=1.000000,G=0.000000,B=0.000000,A=1.000000)" "(R=1.000000,G=0.000000,B=0.177313,A=1.000000)"))
  (if (.bBlockingHit (Collision|BreakHitResult _outhit))
    (bind _outhit_2 (Collision|LineTraceByChannel (Transformation|GetWorldLocation (Variables|Components|GetMuzzle)) (.ImpactPoint (Collision|BreakHitResult _outhit)) "TraceTypeQuery1" false 0 "ForDuration" true "(R=0.096878,G=1.000000,B=0.000000,A=1.000000)"))))