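; Master weapon pickup Blueprint that hands its LinkedWeapon to a PlayerT entering its TriggerBox.
; If the player's SocketUsed flag is already set, it only plays a bounce sound.
; Otherwise it sets the flag, destroys itself with a pickup sound and spawns the weapon attached to the Palm_R socket on the player's Snappoint.
; It also stores the weapon, its class and the pickup's class on the player.
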(event OnComponentBeginOverlap(TriggerBox)
  (params (OverlappedComponent :type Primitive%20Component%20Object%20Reference) (OtherActor :type Actor%20Object%20Reference) (OtherComp :type Primitive%20Component%20Object%20Reference) (OtherBodyIndex :type Integer) (bFromSweep :type Boolean) (SweepResult :type Hit%20Result%20Structure%20%28by%20ref%29))
  (bind _returnvalue (Transformation|GetActorLocation))
  (bind (_asplayer_t _bsuccess) (Utilities|Casting|CastToPlayerT OtherActor))
  (if (Variables|/Game/Character/PlayerT.PlayerT_C|GetSocketUsed _asplayer_t)
    (Audio|PlaySoundatLocation "/Game/Weapons/SciFiWeapDark/Sound/GrenadeLauncher/Wavs/GrenadeLauncher_Bounce04.GrenadeLauncher_Bounce04" _returnvalue "0, 0, 0" 1.0 1.0 0.0 0 0 0)
    (else
      (Variables|/Game/Character/PlayerT.PlayerT_C|SetSocketUsed _asplayer_t true)
      (if _bsuccess
        (Actor|DestroyActor)
        (Audio|PlaySoundatLocation (Variables|Default|GetPickupSound) _returnvalue "0, 0, 0" 1.0 1.0 0.0 0 0 0)
        (bind _returnvalue_2 (Game|SpawnActorfromClass (Variables|Default|GetLinkedWeapon) (Math|Transform|MakeTransform "0, 0, 0" "0, 0, 0" "1,1,1") "Undefined" 0 0))
        (bind _output_get (Variables|/Game/Character/PlayerT.PlayerT_C|SetWeapon _asplayer_t _returnvalue_2))
        (Transformation|AttachComponentToComponent _output_get (Variables|/Game/Character/PlayerT.PlayerT_C|GetSnappoint _asplayer_t) "Palm_R" "KeepRelative" "KeepRelative" "KeepRelative" true)
        (Variables|/Game/Character/PlayerT.PlayerT_C|SetCurrentWeaponPickup _asplayer_t (Utilities|GetClass self))
        (Variables|/Game/Character/PlayerT.PlayerT_C|SetCurrentWeapon _asplayer_t (Variables|Default|GetLinkedWeapon))))))

(fn ConstructionScript)